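; Tank Blueprint that handles orbit-style aiming input and registers its barrel component.
; On BeginPlay it passes TankBarrel to SetBarrelRefrence.
; The AimAzimuth axis yaws the AzimuthGimbal and AimElevation pitches the SpringArm, splitting rotation across two components.
; Both local rotations scale by AimingSpeed and world delta seconds for frame-rate independent movement.
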(event EventBeginPlay
  (Class|Tank|SetBarrelRefrence (Variables|Default|GetTankBarrel)))

(event Input|AxisEvents|InputAxisAimElevation
  (params (AxisValue :type Float%20%28single-precision%29))
  (Transformation|AddLocalRotation (Variables|Default|GetSpringArm) (Math|Rotator|MakeRotator 0.0 (* AxisValue (Utilities|Time|GetWorldDeltaSeconds) (Variables|Default|GetAimingSpeed)) 0.0) false false))

(event Input|AxisEvents|InputAxisAimAzimuth
  (params (AxisValue :type Float%20%28single-precision%29))
  (Transformation|AddLocalRotation (Variables|Default|GetAzimuthGimbal) (Math|Rotator|MakeRotator 0.0 0.0 (* AxisValue (Utilities|Time|GetWorldDeltaSeconds) (Variables|Default|GetAimingSpeed))) false false))

(fn ConstructionScript)